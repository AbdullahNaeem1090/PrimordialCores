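; Gameplay ability that plays a hit-reaction montage on the avatar when activated by a gameplay event.
; It reads the hit result and type from the effect context, then gets hit direction, zone and reaction table from the avatar through message calls.
; These select the montage from the table, and the ability ends when it finishes or is interrupted, or if none is found.
; Debug spheres and prints show each hit.
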(event `self.K2_ActivateAbilityFromEvent`
  (params (EventData :type "GameplayEventData Structure (by ref)"))
  (bind (_eventtag _instigator _target _optionalobject _optionalobject2 _contexthandle) (break `GameplayEventData` EventData))
  (`KismetSystemLibrary.PrintString` (`KismetSystemLibrary.GetDisplayName` _instigator))
  (bind (_outhitresult _outhittype _returnvalue) (`PCBpFunctionLibrary.GetHitResultFromEffectContext` _contexthandle))
  (set `self.Hit Type` _outhittype)
  (if _returnvalue
    (bind (_bblockinghit _binitialoverlap _time _distance _location _impactpoint _normal _impactnormal _physmat _hitactor _hitcomponent _hitbonename) (`GameplayStatics.BreakHitResult` _outhitresult))
    (`KismetSystemLibrary.DrawDebugSphere` _impactpoint 10.0 12 (struct :`R` 0.074825 :`G` 1.0 :`B` 0.068496 :`A` 1.0) 5.0)
    (message `CombatInterface.FillHitReactInfo` (`self.GetAvatarActorFromActorInfo`) _impactpoint _hitbonename (`self.Hit Direction`) (`self.Hit Zone`))
    (bind _returnvalue_2 (message `CombatInterface.GetHitReactDataTable` (`self.GetAvatarActorFromActorInfo`)))
    (bind _returnvalue_3 (`PCBpFunctionLibrary.GetHitReactAnimMontageFromTable` (`self.Hit Type`) (`self.Hit Direction`) (`self.Hit Zone`) _returnvalue_2))
    (`KismetSystemLibrary.PrintString` (`KismetSystemLibrary.GetDisplayName` _returnvalue_3) true true (struct :`R` 1.0 :`G` 0.113155 :`B` 0.036672 :`A` 1.0) 3.0)
    (`KismetSystemLibrary.PrintString` (`|GetEnumeratorNameAsString` (`self.Hit Direction`)) true true (struct :`R` 0.222964 :`G` 0.112306 :`B` 1.0 :`A` 1.0) 3.0)
    (`KismetSystemLibrary.PrintString` (`|GetEnumeratorNameAsString` (`self.Hit Zone`)) true true (struct :`R` 0.084852 :`G` 0.042869 :`B` 1.0 :`A` 1.0) 3.0)
    (`/Engine/EditorBlueprintResources/StandardMacros.IsValid` _returnvalue_3
      (:`Is Valid`
        (`AbilityTask_PlayMontageAndWait.CreatePlayMontageAndWaitProxy` "None" _returnvalue_3
          (:`OnCompleted`
            _)
          (:`OnInterrupted`
            _)
          (:`OnCancelled`
            _))
        (`self.K2_EndAbility`))
      (:`Is Not Valid`
        (`self.K2_EndAbility`)))
    (else
      (`self.K2_EndAbility`))))