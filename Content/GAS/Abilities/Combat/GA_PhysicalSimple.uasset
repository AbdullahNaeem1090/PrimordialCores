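; Gameplay ability for physical melee attacks, picking a light or heavy attack by how long input is held before release.
; Attack data tables supply montage, socket, damage and next combo slot; heavy attacks can motion-warp toward the opponent.
; Montage gameplay events toggle a looping-timer sphere trace that applies damage effects, ignoring actors already hit.
; Pressing input during the combo window queues the next slot's attack, played at the montage end event.
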(event `self.K2_ActivateAbility`
  (`/Engine/EditorBlueprintResources/StandardMacros.IsValid` (`self.GetAvatarActorFromActorInfo`)
    (:`Is Valid`
      (set `self.Avatar Actor` (`self.GetAvatarActorFromActorInfo`))
      (bind (_asynctaskproxy _timeheld) (`AbilityTask_WaitInputRelease.WaitInputRelease` false)
        (:`then`
          ;[0.15 0.15 0.15 0.5 30] Wait Gameplay Events for Trace Start ,Trace Stop , Window Open and close for Combo And End Montage (End montage event is there to for quick attacks)
          (`AbilityTask_WaitGameplayEvent.WaitGameplayEvent` (struct :`TagName` "Event.Trace.Start") null
            (:`then`
              (`AbilityTask_WaitGameplayEvent.WaitGameplayEvent` (struct :`TagName` "Event.Trace.End") null
                (:`then`
                  (`AbilityTask_WaitGameplayEvent.WaitGameplayEvent` (struct :`TagName` "Window.Open") null
                    (:`then`
                      (`AbilityTask_WaitGameplayEvent.WaitGameplayEvent` (struct :`TagName` "Window.Close") null
                        (:`then`
                          (`AbilityTask_WaitGameplayEvent.WaitGameplayEvent` (struct :`TagName` "Montage.End") null
                            (:`EventReceived`
                              (`self.Check And Play Combo`))))
                        (:`EventReceived`
                          (set `self.Is Window Open` false))))
                    (:`EventReceived`
                      (set `self.Is Window Open` true))))
                (:`EventReceived`
                  (`self.Trace Stop`))))
            (:`EventReceived`
              (`self.Trace`))))
        (:`OnRelease`
          (if (> _timeheld (`self.Heavy Attack Threshold Time `))
            ;[0.15 0.15 0.15 0.5 30] Heavy Attack
            (`self.Pre Heavy Attack`)
            (`AbilityTask_PlayMontageAndWait.CreatePlayMontageAndWaitProxy` "None" (`self.Montage to Play`)
              (:`OnCompleted`
                (`self.K2_EndAbility`)))
            (else
              ;[0.15 0.15 0.15 0.5 30] Light Attack
              (`self.Init Or Update Required Variables` (`self.Attack Type Tags`))
              (`AbilityTask_PlayMontageAndWait.CreatePlayMontageAndWaitProxy` "None" (`self.Montage to Play`)
                (:`OnInterrupted`
                  _)
                (:`OnCancelled`
                  _))
              (`self.Trace Stop`))))))
    (:`Is Not Valid`
      (`self.K2_EndAbility`))))

(event `self.OnInputPressed`
  ;[0.15 0.15 0.15 0.5 30] Listens for Input Press (Called From C++)
  (if (`self.Is Window Open`)
    (set `self.Should Play Combo` true)))

(event `Check And Play Combo`
  ;[0.15 0.15 0.15 0.5 30] Plays Next Montage if Window is Open for Combo
  (if (`self.Should Play Combo`)
    (set `self.Should Play Combo` false)
    (bind (_bfound _returnvalue) (`PCBpFunctionLibrary.GetAttackInfoBySlot` "/Game/GAS/Data/DT_Punch.DT_Punch" (`self.Next Attack Slot`)))
    (if _bfound
      (`self.Set Required Varibales ` _returnvalue)
      (`AbilityTask_PlayMontageAndWait.CreatePlayMontageAndWaitProxy` "None" (`self.Montage to Play`)
        (:`OnInterrupted`
          _)
        (:`OnCancelled`
          _))
      (`self.Trace Stop`)
      (else
        (`self.K2_EndAbility`)))
    (else
      (`self.K2_EndAbility`))))

(event `Trace Stop`
  ;[0.15 0.15 0.15 0.5 30] Clearing Timer On trace End
  (`KismetArrayLibrary.Array_Clear` (`self.Actors to Ignore`))
  (`KismetSystemLibrary.K2_ClearAndInvalidateTimerHandle` (`self.Timer Handle`)))

(event `Trace`
  ;[0.15 0.15 0.15 0.5 30] Tracing And Applying Damage
  (set `self.Timer Handle` (struct))
  (bind _returnvalue (`KismetSystemLibrary.K2_SetTimerDelegate` (delegate `Trace Event`) 0.01 true))
  (set `self.Timer Handle` _returnvalue))

(event `Trace Event`
  ;[0.15 0.15 0.15 0.5 30] Tracing And Applying Damage
  (bind _returnvalue (message `CombatInterface.GetSocketLocationByName` (`self.Avatar Actor`) (`self.Attack Socket`)))
  (bind _outhit (`KismetSystemLibrary.SphereTraceSingleForObjects` _returnvalue _returnvalue (`self.Trace Sphere Radius`) (`self.Trace Object Types`) false (`self.Actors to Ignore`) "ForOneFrame"))
  (`self.Post Sphere Trace ` _outhit))

(fn `Init Or Update Required Variables`
  (params (GameplayTags :type "Array of GameplayTag Structure (by ref)"))
  (bind (_bfound _returnvalue) (`PCBpFunctionLibrary.GetRandomAttackInfo` (`self.AttackInfoDataTable`) (`BlueprintGameplayTagLibrary.MakeGameplayTagContainerFromArray` GameplayTags)))
  (if _bfound
    (`self.Set Required Varibales ` _returnvalue)
    (else
      (`self.K2_EndAbility`))))

(fn `Post Sphere Trace `
  (params (HitResult :type "HitResult Structure (by ref)"))
  (locals (`Hit Actor` :type "Actor Object Reference") (`Hit Actor ASC` :type "AbilitySystemComponent Object Reference"))
  (bind (_bblockinghit _binitialoverlap _time _distance _location _impactpoint _normal _impactnormal _physmat _hitactor) (`GameplayStatics.BreakHitResult` HitResult))
  (if _bblockinghit
    (set `local.Hit Actor` _hitactor)
    (set `local.Hit Actor ASC` (`AbilitySystemBlueprintLibrary.GetAbilitySystemComponent` (`local.Hit Actor`)))
    (`KismetArrayLibrary.Array_AddUnique` (`self.Actors to Ignore`) (`local.Hit Actor`))
    (`/Engine/EditorBlueprintResources/StandardMacros.IsValid` (`local.Hit Actor ASC`)
      (:`Is Valid`
        (`PCBpFunctionLibrary.ApplyDamageEffectToTarget` "/Game/GAS/Effects/GE_Test.GE_Test_C" (`self.Avatar Actor`) (`local.Hit Actor ASC`) (`self.Attack Type`) (`local.HitResult`) (`self.Base Damage`))))))

(fn `Pre Heavy Attack`
  (`self.Init Or Update Required Variables` (`self.Attack Type_0`))
  (bind _returnvalue (message `CombatInterface.GetOpponentTarget` (`self.Avatar Actor`)))
  (set `self.Target` _returnvalue)
  (if (`self.Should Do Motion Warping `)
    (message `CombatInterface.UpdateWarpTargetLocation` (`self.Avatar Actor`) (`self.Reduce Vector` 100.0))))

(fn `Reduce Vector`
  (params (`Units Reduction` :type "Float (double-precision)"))
  (returns (`Reduced Vector` :type "Vector Structure"))
  (locals (`Target Vector` :type "Vector Structure" :default (0.0 0.0 0.0)) (`Vector to Subtarct` :type "Vector Structure"))
  (`/Engine/EditorBlueprintResources/StandardMacros.IsValid` (`self.Target`)
    (:`Is Valid`
      (set `local.Target Vector` (`Actor.K2_GetActorLocation` (`self.Target`)))
      (set `local.Vector to Subtarct` (* (`local.Units Reduction`) (`KismetMathLibrary.Normal` (- (`local.Target Vector`) (`Actor.K2_GetActorLocation` (`self.GetAvatarActorFromActorInfo`))))))
      (return (- (`local.Target Vector`) (`local.Vector to Subtarct`))))
    (:`Is Not Valid`
      (`self.K2_EndAbility`))))

(fn `Set Required Varibales `
  (params (NewParam :type "PhysicalAttackData Structure"))
  (locals (`Attack Info` :type "PhysicalAttackData Structure"))
  (bind (_attack_info_attackname _attack_info_attacktype _attack_info_comboslot _attack_info_nextcomboslot _attack_info_basedamage _attack_info_socketname _attack_info_distancerange _attack_info_attackermontage) (break `PhysicalAttackData` (`local.Attack Info`)))
  (set `local.Attack Info` NewParam)
  (set `self.Attack Type` _attack_info_attacktype)
  (set `self.Next Attack Slot` _attack_info_nextcomboslot)
  (set `self.Base Damage` _attack_info_basedamage)
  (set `self.Attack Socket` _attack_info_socketname)
  (bind _output_get (set `self.Montage to Play` _attack_info_attackermontage))
  (set `self.Max Distance from Target` _attack_info_distancerange)
  (`KismetSystemLibrary.PrintString` (`KismetSystemLibrary.GetDisplayName` _output_get)))

(fn `Should Do Motion Warping `
  (returns (ReturnValue :type Boolean))
  (`/Engine/EditorBlueprintResources/StandardMacros.IsValid` (`self.Target`)
    (:`Is Valid`
      (return (> (`self.Max Distance from Target`) (`Actor.GetDistanceTo` (`self.GetAvatarActorFromActorInfo`) (`self.Target`)))))
    (:`Is Not Valid`
      (return false))))