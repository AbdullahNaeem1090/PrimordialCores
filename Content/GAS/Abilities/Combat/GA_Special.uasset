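; GA_Special is a gameplay ability that performs a paired special attack, with synchronized montages on attacker and opponent.
; It checks for paired animation data, target range and facing angle, printing each result for debugging.
; It briefly interpolates to CalculateIdealLocation, whose offset math is left unconnected, then plays both montages.
; The ability ends on failed checks or when the victim montage completes.
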(event `self.K2_ActivateAbility`
  (bind (_pairaniminfo_inputtag _pairaniminfo_attackanim) (break `PairedAnimInfo` (`self.PairAnimInfo`)))
  (bind (_pairaniminfo_inputtag_2 _pairaniminfo_attackanim_2 _pairaniminfo_victimanim) (break `PairedAnimInfo` (`self.PairAnimInfo`)))
  (bind _output_get (set `self.Attacker` (`self.GetAvatarActorFromActorInfo`)))
  (bind _returnvalue (message `CombatInterface.GetOpponentTarget` _output_get))
  (bind _output_get_2 (set `self.Target` _returnvalue))
  (`/Engine/EditorBlueprintResources/StandardMacros.IsValid` _output_get_2
    (:`Is Valid`
      (bind _passed (`self.Check Necessary Conditions`))
      (if _passed
        (`AT_InterpActorLocation.InterpToLocation` (`self.CalculateIdealLocation`) 0.1
          (:`OnFinished`
            (bind _ascharacter (cast `Character` (`self.Target`))
              (:`then`
                (`AbilityTask_PlayMontageAndWait.CreatePlayMontageAndWaitProxy` "None" _pairaniminfo_attackanim
                  (:`then`
                    (`|PlayMontage` (`Character.Mesh` _ascharacter) _pairaniminfo_victimanim
                      (:`OnCompleted`
                        (`self.K2_EndAbility`))))))
              (:`CastFailed`
                (`self.K2_EndAbility`)))))
        (else
          (`self.K2_EndAbility`))))
    (:`Is Not Valid`
      (`self.K2_EndAbility`))))

(fn `Check Necessary Conditions`
  (returns (Passed :type Boolean))
  (bind _returnvalue (`self.IsTargetInIdealRange`))
  (bind (_pairaniminfo_inputtag _pairaniminfo_attackanim _pairaniminfo_victimanim _pairaniminfo_idealdistance _pairaniminfo_distancetolerance _pairaniminfo_minangle _pairaniminfo_maxangle) (break `PairedAnimInfo` (`self.PairAnimInfo`)))
  (bind _returnvalue_2 (`self.TargetIsFacingAttackerInRange` _pairaniminfo_minangle _pairaniminfo_maxangle))
  (bind _returnvalue_3 (`self.GetAndSetPairedAnimInfo`))
  (`KismetSystemLibrary.PrintString` (`KismetStringLibrary.Conv_BoolToString` _returnvalue_3))
  (`KismetSystemLibrary.PrintString` (`KismetStringLibrary.Conv_BoolToString` _returnvalue))
  (`KismetSystemLibrary.PrintString` (`KismetStringLibrary.Conv_BoolToString` _returnvalue_2))
  (return (and _returnvalue_3 _returnvalue _returnvalue_2)))