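; Base enemy character Blueprint that sets up unarmed animation and shows debug information.
; BeginPlay links the unarmed anim layer to the mesh, while Tick prints Health and draws a forward-facing debug arrow every frame.
; A disconnected death sequence would pick a montage from a hit-reaction table by hit type and direction, then switch the mesh to ragdoll physics on blend-out, but it never runs.
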(event `self.ReceiveBeginPlay`
  (`SkeletalMeshComponent.LinkAnimClassLayers` (`self.Mesh`) "/Game/Characters/Locomotion/AnimLayers/ABP_AnimLayer_UnArmed.ABP_AnimLayer_UnArmed_C"))

(event `self.ReceiveTick`
  (params (DeltaSeconds :type "Float (single-precision)"))
  (bind _returnvalue (`self.K2_GetActorLocation`))
  (`KismetSystemLibrary.PrintString` (`KismetStringLibrary.Conv_DoubleToString` (`self.Health`)) true true (struct :`R` 0.063517 :`G` 1.0 :`B` 0.065458 :`A` 1.0) 0.0)
  (`KismetSystemLibrary.DrawDebugArrow` _returnvalue (+ _returnvalue (* (`self.GetActorForwardVector`) (`self.Arrow Size`)))))

(fn `UserConstructionScript`)