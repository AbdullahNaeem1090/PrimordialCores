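; Character locomotion component that switches the owner between gaits and tunes its movement to match.
; UpdateGait records the last and current gait, then sends the new one to the mesh's AnimInstance through a gait data message.
; If that call returns true, it copies speed, acceleration and braking values from the CycleGaitSettings map onto the CharacterMovementComponent.
; BeginPlay sets an initial gait, and a debug key flip-flops between two gaits.
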(event EventBeginPlay
  (CallFunction|UpdateGait "NewEnumerator2"))

(event EventTick
  (params (DeltaSeconds :type Float%20%28single-precision%29)))

(event Input|KeyboardEvents|DebugKey1
  (params (Key :type Key%20Structure) (ActionValue :type Input%20Action%20Value%20Structure))
  (:Pressed
    (Utilities|FlowControl|FlipFlop
      (:A
        (Development|PrintString "Hello")
        (CallFunction|UpdateGait "NewEnumerator1"))
      (:B
        (CallFunction|UpdateGait "NewEnumerator2")))))

(fn UpdateGait
  (params (Desired%20Gait :type E_CycleGaits%20Enum :default "NewEnumerator0"))
  (bind _returnvalue (Components|GetOwner))
  (bind _cycle_gait_settings (Variables|Cycle|GetCycle%20Gait%20Settings))
  (bind _value (Utilities|Map|Find _cycle_gait_settings Desired%20Gait))
  (bind _returnvalue_2 (Actor|GetComponentbyClass _returnvalue "/Script/Engine.CharacterMovementComponent"))
  (bind (_movementspeed _maxaccelration _breakingdecelaration _brakingfrictionfactor _useseparatebrakingfriction _brakingfriction) (Utilities|Struct|BreakST_GaitSettings _value))
  (Variables|Cycle|SetLast%20Cycle%20Gait (Variables|Cycle|GetCurrent%20Cycle%20Gait))
  (Variables|Cycle|SetCurrent%20Cycle%20Gait Desired%20Gait)
  (bind _success (Class|BPIGaitData|RecieveGaitData(Message) (CallFunction|GetAnimInstance) Desired%20Gait))
  (if _success
    (Variables|/Script/Engine.CharacterMovementComponent|SetMaxWalkSpeed _returnvalue_2 _movementspeed)
    (Variables|/Script/Engine.CharacterMovementComponent|SetMaxAcceleration _returnvalue_2 _maxaccelration)
    (Variables|/Script/Engine.CharacterMovementComponent|SetBrakingDecelerationWalking _returnvalue_2 _breakingdecelaration)
    (Variables|/Script/Engine.CharacterMovementComponent|SetBrakingFrictionFactor _returnvalue_2 _brakingfrictionfactor)
    (Variables|/Script/Engine.CharacterMovementComponent|SetbUseSeparateBrakingFriction _returnvalue_2 _useseparatebrakingfriction)
    (Variables|/Script/Engine.CharacterMovementComponent|SetBrakingFriction _returnvalue_2 _brakingfriction)))

(fn GetAnimInstance
  (bind _ascharacter (Utilities|Casting|CastToCharacter (Components|GetOwner))
    (:then
      (return (Components|SkeletalMesh|GetAnimInstance (Variables|/Script/Engine.Character|GetMesh _ascharacter))))
    (:CastFailed
      (return 0))))